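; Test player controller for exercising UMGOverlapControlManager on world widget components, driven by numpad keys.
; BeginPlay adds the manager widget to the viewport; key One spawns TestActors at random positions, caching each widget component and its location and giving it an index.
; Key Two passes the cached components to the manager as a line-align overlap group.
; Key Three moves them back to their cached locations.
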(event `Key|NumPadOne`
  (params (Key :type "Key Structure"))
  (:`Pressed`
    (bind _returnvalue (`|SpawnActorFromClass` "/Game/Testing/TestActor.TestActor_C" (`KismetMathLibrary.MakeTransform` (`KismetMathLibrary.MakeVector` (`KismetMathLibrary.RandomFloatInRange` 0.0 -1200.0) (`KismetMathLibrary.RandomFloatInRange` 0.0 -1200.0))) "Undefined" "MultiplyWithRoot" null null))
    (set `self.NewVar_1` _returnvalue)
    (bind _widget (`/Game/Testing/TestActor.Widget` _returnvalue))
    (bind _returnvalue_2 (`KismetArrayLibrary.Array_Add` (`self.NewVar`) _widget))
    (`KismetArrayLibrary.Array_Add` (`self.NewVar_3`) (`SceneComponent.K2_GetComponentLocation` _widget))
    (bind _aswbp_test_widget (cast `/Game/Testing/WBP_TestWidget` (`WidgetComponent.GetWidget` _widget)))
    (`/Game/Testing/WBP_TestWidget.UpdateIndex` _aswbp_test_widget _returnvalue_2)))

(event `self.ReceiveBeginPlay`
  (`parent.ReceiveBeginPlay`)
  (bind _returnvalue (`|CreateWidget` "/Script/StrangeOverlapMngr.UMGOverlapControlManager"))
  (`UserWidget.AddToViewport` _returnvalue 0)
  (set `self.OverlapManager` _returnvalue))

(event `Key|NumPadTwo`
  (params (Key :type "Key Structure"))
  (:`Pressed`
    (`UMGOverlapControlManager.CreateControlOverlapGroup` (`self.OverlapManager`) (`self.NewVar`) "LineAllign" (`self.Group Tag Id`) (make `UMGOverlapControlGroupSettings` 6))))

(event `Key|NumPadThree`
  (params (Key :type "Key Structure"))
  (:`Pressed`
    (for (_array_element _array_index) (`self.NewVar`)
      (`SceneComponent.K2_SetWorldLocation` _array_element (`|GetArrayItem` (`self.NewVar_3`) _array_index) false false))))

(fn `UserConstructionScript`)